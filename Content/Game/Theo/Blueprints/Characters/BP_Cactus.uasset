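; Cactus character Blueprint that extends a parent character's attack and super attack hooks with a cactus-specific super attack.
; Starting the super plays the nail spell montage if the mesh is visible.
; The trigger, gated by CanSuperAttack, spawns BP_Cactus_Super at the character's transform and calls the ResetSuperAttack dispatcher.
; The handler bound on BeginPlay re-enables the super after a short delay.
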(event Custom|ResetSuperAttack_Event
  (Utilities|FlowControl|Delay 1.0)
  (Variables|Default|SetCanSuperAttack true))

(event EventBeginPlay
  (|CallParentFunction)
  (EventDispatchers|AssignResetSuperAttack (delegate Custom|ResetSuperAttack_Event)))

(fn ConstructionScript)

(fn AttackTrigger
  (|CallParentFunction))

(fn SuperAttackTrigger
  (|CallParentFunction)
  (if (Variables|Default|GetCanSuperAttack)
    (Utilities|FlowControl|Sequence
      (:then_0
        (Variables|Default|SetCanSuperAttack false))
      (:then_1
        (Game|SpawnActorfromClass "/Game/Game/Theo/Blueprints/BP_Cactus_Super.BP_Cactus_Super_C" (Transformation|GetActorTransform) "Undefined" "MultiplyWithRoot" 0 0)
        (Default|CallResetSuperAttack)))))

(fn OnSuperAttackStart
  (|CallParentFunction)
  (if (Rendering|IsVisible (Variables|Character|GetMesh))
    (Utilities|FlowControl|Sequence
      (:then_1
        (Animation|PlayAnimMontage "/Game/Game/Theo/Art/AM_CactusNails_Spell.AM_CactusNails_Spell" 1.0 "None")))))

(fn OnSuperAttackStop
  (|CallParentFunction))