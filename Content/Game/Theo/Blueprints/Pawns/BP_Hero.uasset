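; BP_Hero is a hero container that spawns one actor for each entry in CharacterClasses at its own transform on BeginPlay.
; Its controller possesses the first spawned character, while DisableCharacter turns off capsule collision and hides the mesh on the rest.
; EnableCharacter mirrors that to restore collision and visibility, but its character reference is empty and nothing in this file calls it.
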(event EventBeginPlay
  (for (_array_element _array_index) (Variables|Default|GetCharacterClasses)
    (bind _returnvalue (Game|SpawnActorfromClass _array_element (Transformation|GetActorTransform) "AlwaysSpawn" "MultiplyWithRoot" 0 0))
    (if (== _array_index 0)
      (Pawn|Possess (Pawn|GetController) _returnvalue)
      (else
        (CallFunction|DisableCharacter _returnvalue)))))

(fn ConstructionScript)

(fn DisableCharacter
  (params (Character :type Character%20Object%20Reference))
  (bind _output_get (LocalVariables|SetChar Character))
  (Utilities|IsValid _output_get
    (:Is%20Valid
      (Utilities|FlowControl|Sequence
        (:then_0
          (Collision|SetCollisionEnabled (Variables|/Script/Engine.Character|GetCapsuleComponent (LocalVariables|GetChar)) "NoCollision"))
        (:then_1
          (Rendering|SetVisibility (Variables|/Script/Engine.Character|GetMesh (LocalVariables|GetChar)) false false))))))

(fn EnableCharacter
  (bind _output_get (LocalVariables|SetChar 0))
  (Utilities|IsValid _output_get
    (:Is%20Valid
      (Utilities|FlowControl|Sequence
        (:then_0
          (Collision|SetCollisionEnabled (Variables|/Script/Engine.Character|GetCapsuleComponent (LocalVariables|GetChar)) "QueryAndPhysics"))
        (:then_1
          (Rendering|SetVisibility (Variables|/Script/Engine.Character|GetMesh (LocalVariables|GetChar)) true false))))))