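; BP_FireBullet is a fire bullet Blueprint that marks its target as burnt.
; ApplyEffect sets the target's IsBurnt flag only if it is not already set.
; The event graph and construction script add no logic of their own, and nothing in this Blueprint calls ApplyEffect or handles the burn's consequences.
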(event EventBeginPlay
  (|CallParentFunction) ; This node is disabled and will not be called.\nDrag off pins to build functionality.
)

(event Collision|EventActorBeginOverlap
  (params (OtherActor :type Actor%20Object%20Reference))
  (|CallParentFunction OtherActor) ; This node is disabled and will not be called.\nDrag off pins to build functionality.
)

(event EventTick
  (params (DeltaSeconds :type Float%20%28single-precision%29))
  (|CallParentFunction DeltaSeconds) ; This node is disabled and will not be called.\nDrag off pins to build functionality.
)

(fn ConstructionScript
  (|CallParentFunction))

(fn ApplyEffect
  (params (Target :type BP%20Base%20Character%20Object%20Reference))
  (if (not (Variables|/Game/Game/Theo/Blueprints/Characters/BP_BaseCharacter.BP_BaseCharacter_C|GetIsBurnt Target))
    (Variables|/Game/Game/Theo/Blueprints/Characters/BP_BaseCharacter.BP_BaseCharacter_C|SetIsBurnt Target true)))