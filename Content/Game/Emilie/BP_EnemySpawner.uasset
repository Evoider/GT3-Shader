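; BP_EnemySpawner is an enemy spawner that creates a random class from EnemiesAvailable at a random point inside its SpawnArea box.
; A looping timer started on BeginPlay drives the spawns, adjusting positions for collision or skipping blocked ones.
; Logic to count enemies, pause at a cap and bind OnEnemyDeath, which restarts an inactive timer, is disconnected, so spawning is uncapped.
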(event Custom|SpawnEnemy
  (bind _spawnarea (Variables|Default|GetSpawnArea))
  (bind _returnvalue (Game|SpawnActorfromClass (.OutItem (Utilities|Array|Random (Variables|Default|GetEnemiesAvailable))) (Math|Transform|MakeTransform (Math|Random|RandomPointinBoundingBox (Transformation|GetWorldLocation _spawnarea) (Variables|/Script/Engine.BoxComponent|GetBoxExtent _spawnarea)) "0, 0, 0" "1.000000,1.000000,1.000000") "AdjustIfPossibleButDontSpawnIfColliding" "MultiplyWithRoot" 0 0)))

(event Custom|OnEnemyDeath
  (params (DestroyedActor :type Actor%20Object%20Reference))
  (Variables|Default|SetEnemyNumber (- (Variables|Default|GetEnemyNumber) 1))
  (if (not (Utilities|Time|IsTimerActivebyHandle (Variables|Default|GetSpawnEnemyHandler)))
    (bind _returnvalue (Utilities|Time|SetTimerbyEvent (delegate Custom|SpawnEnemy) 3.0 true))
    (Variables|Default|SetSpawnEnemyHandler _returnvalue)))

(event EventBeginPlay
  (bind _returnvalue (Utilities|Time|SetTimerbyEvent (delegate Custom|SpawnEnemy) 3.0 true))
  (Variables|Default|SetSpawnEnemyHandler _returnvalue))

(fn ConstructionScript)