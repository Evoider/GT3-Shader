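; BP_Turret is an elemental enemy turret with health and a floating health bar widget.
; Its construction script adds a BP_BulletSpawn child actor, passes it the turret's Element, and picks the fire or ice statue material.
; Damage flashes an overlay material on a short timer, updates the health bar and destroys the actor at zero health.
; Tick rotates the widget to face the player camera.
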(event EventTick
  (params (DeltaSeconds :type Float%20%28single-precision%29))
  (bind _widget (Variables|Default|GetWidget))
  (Transformation|SetWorldRotation _widget (Math|Rotator|FindLookatRotation (Transformation|GetWorldLocation _widget) (Transformation|GetWorldLocation (Variables|/Script/Engine.PlayerCameraManager|GetTransformComponent (Game|GetPlayerCameraManager 0)))) false false))

(fn ConstructionScript
  (bind _statue (Variables|Default|GetStatue))
  ;[1 1 1] Add BulletSpawner as child component
  (Utilities|FlowControl|Sequence
    (:then_0
      (bind _returnvalue (AddComponent|AddChildActorComponent false (Math|Conversions|ToTransform(Vector) (Variables|/Script/Engine.SceneComponent|GetRelativeLocation (Variables|Default|GetBulletSpawn)))))
      (ChildActorComponent|SetChildActorClass _returnvalue "/Game/Game/Emilie/BP_BulletSpawn.BP_BulletSpawn_C")
      (bind _asbp_bullet_spawn (Utilities|Casting|CastToBP_BulletSpawn (Variables|/Script/Engine.ChildActorComponent|GetChildActor _returnvalue)))
      (Variables|/Game/Game/Emilie/BP_BulletSpawn.BP_BulletSpawn_C|SetElement _asbp_bullet_spawn (Variables|Default|GetElement)))
    (:then_1
      ;[1 1 1] Set turret material by element
      (switch Utilities|FlowControl|Switch|SwitchonEElement (Variables|Default|GetElement)
        (:NewEnumerator0
          (Rendering|Material|SetMaterial _statue 0 "/Game/Game/Emilie/Materials/M_FireTurret.M_FireTurret"))
        (:NewEnumerator1
          (Rendering|Material|SetMaterial _statue 0 "/Game/Game/Emilie/Materials/M_IceTurret.M_IceTurret"))))))

(fn Damage
  (params (Damage :type Float%20%28double-precision%29))
  (Rendering|Material|SetOverlayMaterial (Variables|Default|GetStatue) "/Game/Game/Emilie/Materials/M_Damage.M_Damage" :!class /Script/Engine.MeshComponent)
  (bind _output_get (Variables|Default|SetCurrentHealth (- (Variables|Default|GetCurrentHealth) Damage)))
  (Utilities|FlowControl|Sequence
    (:then_0
      (bind _ashud_ennemy_health (Utilities|Casting|CastToHUD_EnnemyHealth (UserInterface|GetWidget (Variables|Default|GetWidget))))
      (Default|UpdateHealthBar _ashud_ennemy_health (Variables|Default|GetCurrentHealth)))
    (:then_1
      (Utilities|Time|SetTimerbyEvent (EventDispatchers|CreateEvent :!event ResetOverlay) 0.1))
    (:then_2
      (if (<= _output_get 0.0)
        (Actor|DestroyActor)))))

(fn ResetOverlay
  (Rendering|Material|SetOverlayMaterial (Variables|Default|GetStatue) 0 :!class /Script/Engine.MeshComponent))