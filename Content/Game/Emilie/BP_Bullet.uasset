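; BP_Bullet is a homing projectile that chases the player character and damages any BP_BaseCharacter it overlaps.
; On spawn it adds a scene component to the player and sets it as the projectile movement's homing target.
; On hit it calls ApplyEffect, deals damage and hides, then after a delay calls RemoveEffect and destroys itself.
; Both effect functions are empty here, and the sound spawn is never run.
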(event OnComponentBeginOverlap(Bullet)
  (params (OverlappedComponent :type Primitive%20Component%20Object%20Reference) (OtherActor :type Actor%20Object%20Reference) (OtherComp :type Primitive%20Component%20Object%20Reference) (OtherBodyIndex :type Integer) (bFromSweep :type Boolean) (SweepResult :type Hit%20Result%20Structure%20%28by%20ref%29))
  ;[1 0.2807 0.2708] Destroy Bullet on overlap
  (bind _asbp_base_character (Utilities|Casting|CastToBP_BaseCharacter OtherActor))
  (bind _output_get (Variables|Default|SetTarget _asbp_base_character))
  (CallFunction|ApplyEffect _output_get)
  (Default|Damage (Variables|Default|GetTarget) 5.0 false)
  (Rendering|SetActorHiddenInGame true)
  (Utilities|FlowControl|Delay 5.0)
  (CallFunction|RemoveEffect (Variables|Default|GetTarget))
  (Actor|DestroyActor))

(event EventBeginPlay
  ;[0.6416 0.6747 1] Follow player on spawn
  (bind _asbp_base_character (Utilities|Casting|CastToBP_BaseCharacter (Game|GetPlayerCharacter 0)))
  (bind _returnvalue (AddComponent|AddSceneComponent _asbp_base_character false))
  (Variables|/Script/Engine.ProjectileMovementComponent|SetHomingTargetComponent (Variables|Default|GetProjectileMovement) _returnvalue))

(fn ConstructionScript)

(fn ApplyEffect
  (params (Target :type BP%20Base%20Character%20Object%20Reference)))

(fn RemoveEffect
  (params (Target :type BP%20Base%20Character%20Object%20Reference)))