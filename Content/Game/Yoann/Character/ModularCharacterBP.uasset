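; ModularCharacterBP is a character Blueprint assembled from separate modular mesh parts for hair, gloves, shoes, headgear, shoulder pads, belt and face.
; On BeginPlay, each part takes the main skeletal mesh as its leader pose component, so all of them follow one animated skeleton.
; The shield then snaps to the LeftWeaponShield socket on the glove mesh.
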(event Collision|EventActorBeginOverlap
  (params (OtherActor :type Actor%20Object%20Reference)))

(event EventTick
  (params (DeltaSeconds :type Float%20%28single-precision%29)))

(event EventBeginPlay
  (Components|SkinnedMesh|SetLeaderPoseComponent (Variables|Default|GetHair) (Variables|SkeletalMeshActor|GetSkeletalMeshComponent) true false)
  (Transformation|AttachComponentToComponent (Variables|Default|GetShield) (Variables|Default|GetGlove) "LeftWeaponShield" "SnapToTarget" "SnapToTarget" "SnapToTarget" true))

(fn ConstructionScript)