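; BP_CrystalDestructibleWall is a breakable crystal wall built on a Chaos Geometry Collection.
; On BeginPlay it takes a random yaw and anchors the collection's first piece by index.
; The first Chaos break event, guarded by IsBroken, prints a debug counter, disables both capsule collisions and destroys the actor after a short delay.
; Construction-script logic for registering an anchor field child actor is disconnected and never runs.
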(event OnChaosBreakEvent(SM_crystal_group_02_GeometryCollection)
  (params (BreakEvent :type Chaos%20Break%20Event%20Structure%20%28by%20ref%29))
  (bind _c (Variables|Default|Getc))
  (if (not (Variables|Default|GetIsBroken))
    (Math|Integer|IncrementInt _c
      (:%20%20
        (Development|PrintString (Utilities|String|ToString(Integer) _c))
        (Variables|Default|SetIsBroken true)
        (Collision|SetCollisionEnabled (Variables|Default|GetCapsule) "NoCollision")
        (Collision|SetCollisionEnabled (Variables|Default|GetCapsule1) "NoCollision")
        (Utilities|FlowControl|Delay 3.0)
        (Actor|DestroyActor)))))

(event EventBeginPlay
  (Transformation|SetActorRotation (Math|Rotator|MakeRotator 0.0 0.0 (Math|Random|RandomFloatinRange 0.0 3.6e+02)) true)
  (Class|GeometryCollectionComponent|SetAnchoredbyIndex (Variables|Default|GetSM_crystal_group_02_GeometryCollection) 0 true))

(fn ConstructionScript)