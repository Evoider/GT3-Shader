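; Crystal projectile built on a Geometry Collection that reacts to Chaos physics collisions.
; Hits on a BP_Enemy apply a small fixed damage on every collision event, with no one-shot guard.
; The first hit on anything else spawns a BP_FS_Projectile actor at the impact location and sets IsBroken, so it spawns only once.
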(event OnChaosPhysicsCollision(SM_crystal_01_GeometryCollection)
  (params (CollisionInfo :type Chaos%20Physics%20Collision%20Info%20Structure%20%28by%20ref%29))
  (bind _asbp_enemy (Utilities|Casting|CastToBP_Enemy (Components|GetOwner (.othercomponent CollisionInfo)))
    (:then
      (Game|Damage|ApplyDamage _asbp_enemy 1.0 0 0))
    (:CastFailed
      (if (not (Variables|Default|GetIsBroken))
        (Game|SpawnActorfromClass "/Game/Game/Yoann/BP_FS_Projectile.BP_FS_Projectile_C" (Math|Conversions|ToTransform(Vector) (.location CollisionInfo)) "Undefined" "MultiplyWithRoot" 0 0)
        (Variables|Default|SetIsBroken true)))))

(event EventBeginPlay)

(event Collision|EventActorBeginOverlap
  (params (OtherActor :type Actor%20Object%20Reference)))

(event EventTick
  (params (DeltaSeconds :type Float%20%28single-precision%29)))

(fn ConstructionScript)