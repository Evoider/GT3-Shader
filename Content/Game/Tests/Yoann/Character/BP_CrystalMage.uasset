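; Crystal Mage character Blueprint with a wand attack and a Crystal Wave super attack, plus modular mesh parts following the main skeleton.
; The attack traces from the camera and fires a projectile and Chaos shoot force from the wand toward the aim point.
; The super samples a spawned preview sphere's position on a timer, then on release or timeout builds the wave's spline from those points.
; An earlier forward-stepping heal-spawn version remains, untriggered here.
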(event Custom|First%20Try%20wave
  ;[0.004322 0 0.02083] Another version to get Points
  (if (<= (Variables|Default|GetCurrentPoint) (Variables|Default|GetMaxNuberOfPoint))
    (Utilities|Time|SetTimerbyEvent (delegate Custom|First%20try%20wave%20get%20point) 0.2)
    (else
      (Variables|Default|SetCurrentPoint 0)
      (for _index (range 0 (- (Utilities|Map|Length (Variables|Default|GetCrystalPoints)) 1))
        (Game|SpawnActorfromClass "/Game/ThirdParty/Stylized_VFX_StPack/Blueprints/BP_Heallvl1.BP_Heallvl1_C" (Math|Conversions|ToTransform(Vector) (.Value (Utilities|Map|Find (Variables|Default|GetCrystalPoints) _index))) "Undefined" "MultiplyWithRoot" 0 0))
      (Utilities|Map|Clear (Variables|Default|GetCrystalPoints)))))

(event Custom|First%20try%20wave%20get%20point
  ;[0.004322 0 0.02083] Another version to get Points
  (if (== (Variables|Default|GetCurrentPoint) 0)
    (Utilities|Map|Add (Variables|Default|GetCrystalPoints) 0 (+ (* (Transformation|GetActorForwardVector) 5e+01) (Transformation|GetActorLocation)))
    (else
      (Utilities|Map|Add (Variables|Default|GetCrystalPoints) (Variables|Default|GetCurrentPoint) (+ (.Value (Utilities|Map|Find (Variables|Default|GetCrystalPoints) (- (Variables|Default|GetCurrentPoint) 1))) (* (Transformation|GetActorForwardVector) 2e+02)))))
  (Variables|Default|SetCurrentPoint (+ (Variables|Default|GetCurrentPoint) 1))
  (CallFunction|FirstTryWave))

(event Custom|AddPoint
  (bind _previewsphere (Variables|Default|GetPreviewSphere)
    (:then
      (Utilities|Map|Add (Variables|Default|GetCrystalPoints) (Variables|Default|GetCurrentPoint) (- (Transformation|GetActorLocation _previewsphere) "0.000000,0.000000,100.000000"))
      (Math|Integer|IncrementInt (Variables|Default|GetCurrentPoint)))
    (:else)))

(event Custom|spawn%20Crystal%20Wave
  ;[0.00619 0 0.02083] Crystal Wave
  (if (not (Variables|Default|GetIsCrystalWaveSpawned))
    (bind _previewsphere (Variables|Default|GetPreviewSphere)
      (:then
        (Actor|DestroyActor _previewsphere)
        (Utilities|Time|ClearandInvalidateTimerbyHandle (Variables|Default|GetGetSpherePointTimer))
        (Variables|Default|SetCurrentPoint 0)
        (bind _returnvalue (Game|SpawnActorfromClass "/Game/Game/Tests/Yoann/Niagara/BP_CrystalWave.BP_CrystalWave_C" (Math|Conversions|ToTransform(Vector) (.Value (Utilities|Map|Find (Variables|Default|GetCrystalPoints) 0))) "Undefined" "MultiplyWithRoot" 0 0))
        (Variables|Default|SetCrystalWaveSpline (Variables|/Game/Game/Tests/Yoann/Niagara/BP_CrystalWave.BP_CrystalWave_C|GetSpline _returnvalue))
        (for _index (range 0 (- (Utilities|Map|Length (Variables|Default|GetCrystalPoints)) 1))
          (Spline|AddSplinePoint (Variables|Default|GetCrystalWaveSpline) (.Value (Utilities|Map|Find (Variables|Default|GetCrystalPoints) _index)) "World" true)
          (Variables|Default|SetIsCrystalWaveSpawned true))
        (Utilities|Map|Clear (Variables|Default|GetCrystalPoints)))
      (:else))))

(event Input|EnhancedActionEvents|EnhancedInputActionIA_TowerAttack_SuperAttack
  (params (ActionValue :type Boolean) (ElapsedSeconds :type Float%20%28double-precision%29) (TriggeredSeconds :type Float%20%28double-precision%29) (InputAction :type Input%20Action%20Object%20Reference :default "/Game/Game/Tests/Theo/Inputs/Actions/IA_TowerAttack_SuperAttack.IA_TowerAttack_SuperAttack"))
  (bind _returnvalue (Transformation|GetActorLocation))
  (:Started
    (Variables|Default|SetIsCrystalWaveSpawned false)
    (Utilities|Map|Add (Variables|Default|GetCrystalPoints) (Variables|Default|GetCurrentPoint) (- _returnvalue "0.000000,0.000000,100.000000"))
    (bind _returnvalue_2 (Game|SpawnActorfromClass "/Game/Game/Tests/Yoann/BP_PreviewSphere.BP_PreviewSphere_C" (Math|Conversions|ToTransform(Vector) _returnvalue) "Undefined" "MultiplyWithRoot" 0 0))
    (Variables|Default|SetPreviewSphere _returnvalue_2)
    (bind _returnvalue_3 (Utilities|Time|SetTimerbyEvent (delegate Custom|AddPoint) 0.1 true))
    (Variables|Default|SetGetSpherePointTimer _returnvalue_3)
    (Utilities|FlowControl|Delay 1.5)
    (CallFunction|SpawnCrystalWave))
  (:Completed
    (CallFunction|SpawnCrystalWave)))

(event Input|EnhancedActionEvents|EnhancedInputActionIA_TowerAttack_Attack
  (params (ActionValue :type Boolean) (ElapsedSeconds :type Float%20%28double-precision%29) (TriggeredSeconds :type Float%20%28double-precision%29) (InputAction :type Input%20Action%20Object%20Reference :default "/Game/Game/Tests/Theo/Inputs/Actions/IA_TowerAttack_Attack.IA_TowerAttack_Attack"))
  (bind _camera (Variables|Default|GetCamera))
  (bind _wand03sm (Variables|Default|GetWand03SM))
  (bind _returnvalue (Transformation|GetWorldLocation _wand03sm))
  (bind _returnvalue_2 (Transformation|GetWorldLocation _camera))
  (bind (_outhit _returnvalue_3) (Collision|LineTraceByChannel _returnvalue_2 (+ _returnvalue_2 (* (Math|Vector|GetForwardVector _camera) 1e+04)) "TraceTypeQuery1" false 0 "None"))
  (Game|SpawnActorfromClass "/Game/Game/Tests/Yoann/Chaos/Projectile/BP_CrsytalProjectile.BP_CrsytalProjectile_C" (Math|Transform|MakeTransform _returnvalue (Math|Rotator|FindLookatRotation _returnvalue (Math|Vector|SelectVector (.Location (Collision|BreakHitResult _outhit)) (.TraceEnd (Collision|BreakHitResult _outhit)) _returnvalue_3))) "Undefined" "MultiplyWithRoot" 0 0)
  (bind _returnvalue_4 (Game|SpawnActorfromClass "/Game/Game/Tests/Yoann/Chaos/Projectile/ChaosShootForce.ChaosShootForce_C" (Math|Transform|MakeTransform _returnvalue (Math|Rotator|FindLookatRotation _returnvalue (Math|Vector|SelectVector (.Location (Collision|BreakHitResult _outhit)) (.TraceEnd (Collision|BreakHitResult _outhit)) _returnvalue_3))) "Undefined" "MultiplyWithRoot" 0 0))
  (Default|FireandDestroy _returnvalue_4))

(event EventBeginPlay
  (Components|SkinnedMesh|SetLeaderPoseComponent (Variables|Default|GetGlove03SK) (Variables|Character|GetMesh) true false))

(fn ConstructionScript)

(fn CreateCrystalPoint
  (params (Key :type Integer%20%28by%20ref%29)))