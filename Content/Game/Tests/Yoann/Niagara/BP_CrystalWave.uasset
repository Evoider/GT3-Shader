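; Test Blueprint that grows a wave of crystals along a spline, paired with a Niagara effect.
; BeginPlay passes loop and spawn counts to Niagara and starts a fast looping timer that calls AddCrystal.
; Each call adds a child actor at the next spline point with random yaw and a scale proportional to its index, starting at zero.
; Once every point is filled, IsDone is set and Tick clears the timer.
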(event EventBeginPlay
  (Class|NiagaraComponent|SetVariableInt (Variables|Default|GetNiagara) "LoopCount" (Variables|Default|GetLoopCount))
  (Class|NiagaraComponent|SetVariableInt (Variables|Default|GetNiagara) "SpawnCount" (Variables|Default|GetSpawnCount))
  (bind _returnvalue (Utilities|Time|SetTimerbyFunctionName 0 "AddCrystal" 0.05 true))
  (Variables|Default|SetAddCrystalTimer _returnvalue))

(event EventTick
  (params (DeltaSeconds :type Float%20%28single-precision%29))
  (if (Variables|Default|GetIsDone)
    (Utilities|Time|ClearandInvalidateTimerbyHandle (Variables|Default|GetAddCrystalTimer))))

(fn ConstructionScript)

(fn AddCrystal
  (bind _totalcrystals (Variables|Default|GetTotalCrystals))
  (if (not (Variables|Default|GetIsDone))
    (AddComponent|AddChildActorComponent false (Math|Transform|MakeTransform (Spline|GetLocationatSplinePoint (Variables|Default|GetSpline) _totalcrystals "Local") (Math|Rotator|MakeRotator 0.0 0.0 (Math|Random|RandomFloatinRange 0.0 3.6e+02)) (* "0.500000,0.500000,0.500000" _totalcrystals)))
    (bind _result (Math|Integer|IncrementInt (Variables|Default|GetTotalCrystals))
      (:%20%20
        (if (== _result (Spline|GetNumberOfSplinePoints (Variables|Default|GetSpline)))
          (Variables|Default|SetIsDone true))))))