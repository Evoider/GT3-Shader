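; Test player character that can fire a super-attack projectile and damage enemies with its right-hand weapon.
; BeginPlay makes the hair, glove, shoe, face and shoulder pad meshes follow the main skeletal mesh's pose.
; The super-attack input spawns BP_MattProjectile ahead of the actor along its forward vector.
; Weapon hits apply fixed damage to BP_Enemy actors, with weapon collision set to probe on BeginPlay and query-only on possess or unpossess.
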(event OnComponentHit(RightWeapon)
  (params (HitComponent :type Primitive%20Component%20Object%20Reference) (OtherActor :type Actor%20Object%20Reference) (OtherComp :type Primitive%20Component%20Object%20Reference) (NormalImpulse :type Vector :default "0, 0, 0") (Hit :type Hit%20Result%20Structure%20%28by%20ref%29))
  (bind _asbp_enemy (Utilities|Casting|CastToBP_Enemy OtherActor))
  (Game|Damage|ApplyDamage _asbp_enemy 1e+01 0 0))

(event Input|EnhancedActionEvents|EnhancedInputActionIA_TowerAttack_SuperAttack
  (params (ActionValue :type Boolean) (ElapsedSeconds :type Float%20%28double-precision%29) (TriggeredSeconds :type Float%20%28double-precision%29) (InputAction :type Input%20Action%20Object%20Reference :default "/Game/Game/Tests/Theo/Inputs/Actions/IA_TowerAttack_SuperAttack.IA_TowerAttack_SuperAttack"))
  (bind _self self)
  (bind _returnvalue (Transformation|GetActorForwardVector _self))
  (Game|SpawnActorfromClass "/Game/Game/Tests/Matt/Character/Projectile/BP_MattProjectile.BP_MattProjectile_C" (Math|Transform|MakeTransform (+ (Transformation|GetActorLocation) (* _returnvalue 2e+02)) (Math|Conversions|RotationFromXVector _returnvalue)) "AlwaysSpawn" "MultiplyWithRoot" 0 0))

(event EventBeginPlay
  (Components|SkinnedMesh|SetLeaderPoseComponent (Variables|Default|GetHair) (Variables|Default|GetSkeletal%20Mesh%20Component) true false)
  (Collision|SetCollisionEnabled (Variables|Default|GetRightWeapon) "QueryAndProbe"))

(event EventPossessed
  (params (NewController :type Controller%20Object%20Reference))
  (Collision|SetCollisionEnabled (Variables|Default|GetRightWeapon) "QueryOnly"))

(event EventUnpossessed
  (params (OldController :type Controller%20Object%20Reference))
  (Collision|SetCollisionEnabled (Variables|Default|GetRightWeapon) "QueryOnly"))

(fn ConstructionScript
  (|CallParentFunction))

(fn NewFunction)