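; Test enemy character that chases the hero controller with AI MoveTo on Tick, switching to a still-empty Attack within attacking range.
; Damage lowers Life and sets a hit flag; at zero it flags death, stops movement and ignores selected collision channels.
; A custom event turns it toward a destination after a tiny workaround delay and launches it there on a suggested projectile arc.
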(event Custom|CustomEvent
  (params (Destination :type Vector))
  (bind (_x _y _z) (Math|Vector|BreakVector Destination))
  (Utilities|FlowControl|Sequence
    (:then_0
      ;[1 1 1] Doesn't work without it
      (Utilities|FlowControl|Delay 0.01)
      (Transformation|SetActorRotation (Math|Rotator|MakeRotator 0.0 0.0 (.yaw (Math|Rotator|FindLookatRotation (Transformation|GetActorLocation) Destination)))))
    (:then_1
      (bind _outlaunchvelocity (Game|SuggestProjectileVelocityCustomArc (Transformation|GetActorLocation) (Math|Vector|MakeVector _x _y (+ _z 2e+02)) 0.0 0.5))
      (Character|LaunchCharacter _outlaunchvelocity true true))))

(event EventBeginPlay
  (bind _asbp_hero_controller (Utilities|Casting|CastToBP_HeroController (Game|GetPlayerController 0)))
  (Variables|Default|SetAs%20BP%20Hero%20Controller _asbp_hero_controller))

(event EventTick
  (params (DeltaSeconds :type Float%20%28single-precision%29))
  (if (<= (Transformation|GetDistanceTo (Variables|Default|GetAs%20BP%20Hero%20Controller)) (+ (Variables|Default|GetAttackingRange) 1e+02))
    (CallFunction|Attack)
    (else
      (AI|AIMoveTo self "0, 0, 0" (Variables|Default|GetAs%20BP%20Hero%20Controller) 5.0 false))))

(event Game|Damage|EventAnyDamage
  (params (Damage :type Float%20%28single-precision%29) (DamageType :type Damage%20Type%20Object%20Reference) (InstigatedBy :type Controller%20Object%20Reference) (DamageCauser :type Actor%20Object%20Reference))
  (CallFunction|UpdateLife Damage)
  (Variables|Default|SetIsHit true))

(event Collision|EventActorBeginOverlap
  (params (OtherActor :type Actor%20Object%20Reference)))

(fn ConstructionScript)

(fn UpdateLife
  (params (Value :type Float%20%28double-precision%29))
  (bind _output_get (Variables|Default|SetLife (- (Variables|Default|GetLife) Value)))
  (if (<= _output_get 0.0)
    (CallFunction|Die)))

(fn Die
  (Variables|Default|SetIsDead true)
  (Class|NavMovementComponent|StopActiveMovement (Variables|Character|GetCharacterMovement))
  (CallFunction|DeactivateCollision))

(fn DeactivateCollision
  (Collision|SetCollisionResponsetoChannel (Variables|Collision|GetCapsuleComponent) "ECC_GameTraceChannel1" "ECR_Ignore")
  (Collision|SetCollisionResponsetoChannel (Variables|Character|GetMesh) "ECC_WorldStatic" "ECR_Ignore")
  (Collision|SetCollisionResponsetoChannel (Variables|Collision|GetCapsuleComponent) "ECC_Pawn" "ECR_Ignore")
  (Collision|SetCollisionResponsetoChannel (Variables|Character|GetMesh) "ECC_Pawn" "ECR_Ignore"))

(fn Attack)