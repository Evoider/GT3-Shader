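; BP_BulletSpawn is a turret-style actor that shoots fire or ice bullets at a BP_BaseCharacter entering its aggro area.
; On BeginPlay, its Element selects the bullet class and Niagara orb effect.
; A looping timer, offset to fire immediately, snaps it toward the target and plays the effect as a cast.
; After a delay it spawns a bullet at the Arrow if the target remains close; any end overlap pauses the timer.
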(event OnComponentBeginOverlap(AggroArea)
  (params (OverlappedComponent :type Primitive%20Component%20Object%20Reference) (OtherActor :type Actor%20Object%20Reference) (OtherComp :type Primitive%20Component%20Object%20Reference) (OtherBodyIndex :type Integer) (bFromSweep :type Boolean) (SweepResult :type Hit%20Result%20Structure%20%28by%20ref%29))
  ;[1 1 1] Triggers when target enter and exit aggro area
  (bind _asbp_base_character (Utilities|Casting|CastToBP_BaseCharacter OtherActor))
  (Variables|Default|SetTarget _asbp_base_character)
  (Variables|Default|SetTargetIsClose true)
  (bind _returnvalue (Utilities|Time|SetTimerbyEvent (delegate Custom|ShootPlayer) 4.0 true -4.0)))

(event OnComponentEndOverlap(AggroArea)
  (params (OverlappedComponent :type Primitive%20Component%20Object%20Reference) (OtherActor :type Actor%20Object%20Reference) (OtherComp :type Primitive%20Component%20Object%20Reference) (OtherBodyIndex :type Integer))
  ;[1 1 1] Triggers when target enter and exit aggro area
  (Utilities|FlowControl|Sequence
    (:then_0
      (if (Components|Activation|IsActive (Variables|Default|GetNiagara))
        (Utilities|FlowControl|Delay 0.2)
        (Components|Activation|Deactivate (Variables|Default|GetNiagara))))
    (:then_1
      (Variables|Default|SetTargetIsClose false)
      (Utilities|Time|PauseTimerbyHandle (stale OnComponentBeginOverlap(AggroArea) _returnvalue)))))

(event Custom|ShootPlayer
  ;[1 1 1] Follow target to shoot
  (Transformation|SetActorRotation (Math|Rotator|FindLookatRotation (Transformation|GetActorLocation) (Transformation|GetActorLocation (Variables|Default|GetTarget))))
  ;[1 1 1] Shoot target after cast if target is still close
  (Components|Activation|Activate (Variables|Default|GetNiagara) false)
  (Utilities|FlowControl|Delay 2.0)
  (if (Variables|Default|GetTargetIsClose)
    (Game|SpawnActorfromClass (Variables|Default|GetBulletType) (Transformation|GetWorldTransform (Variables|Default|GetArrow)) "Undefined" "MultiplyWithRoot" 0 0)
    (Components|Activation|Deactivate (Variables|Default|GetNiagara))))

(event EventBeginPlay
  ;[1 1 1] Set element to bullets and niagara
  (switch Utilities|FlowControl|Switch|SwitchonEElement (Variables|Default|GetElement)
    (:NewEnumerator0
      (Variables|Default|SetBulletType "/Game/Game/Tests/Emilie/BP_FireBullet.BP_FireBullet_C")
      (Class|NiagaraComponent|SetAsset (Variables|Default|GetNiagara) "/Game/Game/Tests/Emilie/Niagara/NS_FireOrbs.NS_FireOrbs" true))
    (:NewEnumerator1
      (Variables|Default|SetBulletType "/Game/Game/Tests/Emilie/BP_IceBullet.BP_IceBullet_C")
      (Class|NiagaraComponent|SetAsset (Variables|Default|GetNiagara) "/Game/Game/Tests/Emilie/Niagara/NS_IceOrbs.NS_IceOrbs" true))))

(fn ConstructionScript)