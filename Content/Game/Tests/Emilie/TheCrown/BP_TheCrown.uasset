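; BP_TheCrown is a character Blueprint for "The Crown", built from modular skeletal mesh parts and kept in a test folder.
; On BeginPlay it runs the parent logic, makes the hair, glove, shoe, face and headgear meshes follow the main skeletal mesh through leader pose, then sets its name.
; The construction script only calls the parent, and this Blueprint's graphs add no other behavior.
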(event EventBeginPlay
  (|CallParentFunction)
  (Components|SkinnedMesh|SetLeaderPoseComponent (Variables|Default|GetHair) (Variables|Default|GetSkeletal%20Mesh%20Component) false false)
  (Variables|Default|SetName "The Crown"))

(fn ConstructionScript
  (|CallParentFunction))