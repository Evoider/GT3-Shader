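; Ice bullet Blueprint that applies and removes a freeze status effect on a target.
; ApplyEffect sets the target's IsFrozen flag if it is not already set, then calls FreezeCharacter on its BP_HeroController.
; RemoveEffect clears the flag and calls UnfreezeCharacter on that controller.
; The event graph holds only disabled placeholders, so this file contains no movement, hit or timing logic.
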(event EventBeginPlay
  (|CallParentFunction) ; This node is disabled and will not be called.\nDrag off pins to build functionality.
)

(event Collision|EventActorBeginOverlap
  (params (OtherActor :type Actor%20Object%20Reference)))

(event EventTick
  (params (DeltaSeconds :type Float%20%28single-precision%29)))

(fn ConstructionScript
  (|CallParentFunction))

(fn ApplyEffect
  (params (Target :type BP%20Base%20Character%20Object%20Reference))
  (if (not (Variables|/Game/Game/Tests/Theo/Blueprints/Characters/BP_BaseCharacter.BP_BaseCharacter_C|GetIsFrozen Target))
    (Variables|/Game/Game/Tests/Theo/Blueprints/Characters/BP_BaseCharacter.BP_BaseCharacter_C|SetIsFrozen Target true)
    (bind _asbp_hero_controller (Utilities|Casting|CastToBP_HeroController (Pawn|GetController Target)))
    (Default|FreezeCharacter _asbp_hero_controller)))

(fn RemoveEffect
  (params (Target :type BP%20Base%20Character%20Object%20Reference))
  (Variables|/Game/Game/Tests/Theo/Blueprints/Characters/BP_BaseCharacter.BP_BaseCharacter_C|SetIsFrozen Target false)
  (bind _asbp_hero_controller (Utilities|Casting|CastToBP_HeroController (Pawn|GetController Target)))
  (Default|UnfreezeCharacter _asbp_hero_controller))