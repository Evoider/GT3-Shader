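; Base hero character for the Tower Attack mode, registering with the game mode and binding overridable attack and super-attack hooks to the hero controller's events.
; Normal attack start fires only while possessed.
; Damage reduces life and briefly flashes an overlay across all meshes before restoring the burn, freeze or default look; death notifies listeners and swaps characters through the controller.
; Tick manages burning as a timed, looping damage effect.
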(event Custom|OnAttackStart_Event
  (if (Variables|Default|GetPossessed)
    (CallFunction|OnAttackStart)))

(event Custom|OnAttackStop_Event
  (CallFunction|OnAttackStop))

(event Custom|OnSuperAttackStart_Event
  (CallFunction|OnSuperAttackStart))

(event Custom|OnSuperAttackStop_Event
  (CallFunction|OnSuperAttackStop))

(event Custom|Burning
  (CallFunction|Damage 2.0 true))

(event EventBeginPlay
  (Utilities|FlowControl|Sequence
    (:then_0
      (bind _asbp_hero_controller (Utilities|Casting|CastToBP_HeroController (Game|GetPlayerController 0)))
      (Variables|Default|SetHeroController _asbp_hero_controller)
      (Utilities|FlowControl|Sequence
        (:then_0
          (EventDispatchers|AssignOnAttackStart _asbp_hero_controller (delegate Custom|OnAttackStart_Event))
          (EventDispatchers|AssignOnAttackStop _asbp_hero_controller (delegate Custom|OnAttackStop_Event)))
        (:then_1
          (EventDispatchers|AssignOnSuperAttackStart _asbp_hero_controller (delegate Custom|OnSuperAttackStart_Event))
          (EventDispatchers|AssignOnSuperAttackStop _asbp_hero_controller (delegate Custom|OnSuperAttackStop_Event)))
        (:then_2
          (Variables|Default|SetDefaultRunSpeed (Variables|/Game/Game/Tests/Theo/Blueprints/Controllers/BP_HeroController.BP_HeroController_C|GetCurrentRunSpeed _asbp_hero_controller)))))
    (:then_1
      (bind _asgm_tower_attack (Utilities|Casting|CastToGM_TowerAttack (Game|GetGameMode)))
      (Default|AddCharacter _asgm_tower_attack self))))

(event Game|Damage|EventAnyDamage
  (params (Damage :type Float%20%28single-precision%29) (DamageType :type Damage%20Type%20Object%20Reference) (InstigatedBy :type Controller%20Object%20Reference) (DamageCauser :type Actor%20Object%20Reference))
  (CallFunction|Damage Damage false))

(event EventTick
  (params (DeltaSeconds :type Float%20%28single-precision%29))
  (if (Utilities|Time|IsTimerActivebyHandle (Variables|Default|GetBurningHandle))
    (if (not (Variables|Default|GetIsBurnt))
      (Utilities|Time|PauseTimerbyHandle (Variables|Default|GetBurningHandle) :!label _label)
      (CallFunction|SetOverlayMaterialtoAllMesh))
    (elif (Variables|Default|GetIsBurnt)
      (bind _returnvalue (Utilities|Time|SetTimerbyEvent (delegate Custom|Burning) 1.0 true))
      (Variables|Default|SetBurningHandle _returnvalue)
      (CallFunction|SetOverlayMaterialtoAllMesh)
      (Utilities|FlowControl|Delay 5.0)
      (Variables|Default|SetIsBurnt false)
      (goto _label))))

(event EventPossessed
  (params (NewController :type Controller%20Object%20Reference))
  (Variables|Default|SetPossessed true))

(event EventUnpossessed
  (params (OldController :type Controller%20Object%20Reference))
  (Variables|Default|SetPossessed false))

(fn ConstructionScript)

(fn OnAttackStart
  (Development|PrintString "OnAttackStart")
  (Development|PrintString (Variables|Default|GetName)))

(fn OnAttackStop)

(fn OnSuperAttackStart)

(fn OnSuperAttackStop)

(fn AttackTrigger
  (Development|PrintString "Attack Trigger"))

(fn SuperAttackTrigger)

(fn Damage
  (params (Damage :type Float%20%28double-precision%29) (EffectDamage :type Boolean))
  (if (not (or (Variables|Character|GetDead) (and (Variables|Default|GetIsTakingDamage) (not EffectDamage))))
    (CallFunction|SetOverlayMaterialtoAllMesh "/Game/Game/Tests/Emilie/Materials/M_Damage.M_Damage")
    (bind _output_get (Variables|Character|SetCurrentLife (- (Variables|Character|GetCurrentLife) Damage)))
    (Utilities|FlowControl|Sequence
      (:then_0
        (Utilities|Time|SetTimerbyEvent (EventDispatchers|CreateEvent :!event OnDamageEnd) 0.1))
      (:then_1
        (if (<= _output_get 0.0)
          (CallFunction|Death))))))

(fn Death
  (Variables|Character|SetDead true)
  (Audio|PlaySound2D "/Game/StarterRessources/StarterContent/Audio/Explosion01.Explosion01" 1.0 1.0 0.0 0 0)
  (Default|CallOnDeath self)
  (bind _asbp_hero_controller (Utilities|Casting|CastToBP_HeroController (Game|GetPlayerController 0)))
  (Default|SwapCharacter _asbp_hero_controller true))

(fn OnDamageEnd
  (Variables|Default|SetIsTakingDamage false)
  (if (Variables|Default|GetIsBurnt)
    (CallFunction|SetOverlayMaterialtoAllMesh "/Game/Game/Tests/Alexis/Material/Fire/M_FireOverlay2.M_FireOverlay2")
    (elif (Variables|Default|GetIsFrozen)
      (CallFunction|SetOverlayMaterialtoAllMesh "/Game/Game/Tests/Alexis/Material/Ice_Snow/M_IceOverlay.M_IceOverlay")
      (else
        (CallFunction|SetOverlayMaterialtoAllMesh)))))

(fn SetOverlayMaterialtoAllMesh
  (params (OverlayMaterial :type Material%20Object%20Reference))
  (bind _mesh (Variables|Character|GetMesh))
  (Utilities|FlowControl|Sequence
    (:then_0
      (Rendering|Material|SetOverlayMaterial _mesh OverlayMaterial :!class /Script/Engine.MeshComponent))
    (:then_1
      (for _array_element (Components|GetChildrenComponents _mesh true)
        (bind _asmesh_component (Utilities|Casting|CastToMeshComponent _array_element))
        (Rendering|Material|SetOverlayMaterial _asmesh_component OverlayMaterial :!class /Script/Engine.MeshComponent)))))