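; Tower-attack game mode that tracks win and loss by watching turrets and characters in the level.
; On BeginPlay it creates the health HUD, gathers all turrets and base characters, and binds to their destroy and death events.
; Each event removes the actor from its array; an empty turret list only logs a win, while an empty character list prints game over and resets the level.
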(event Custom|OnCharacterDeath
  (params (Character :type BP%20Base%20Character%20Object%20Reference))
  (bind _characters (Variables|Default|GetCharacters))
  (Utilities|Array|RemoveItem _characters Character)
  (if (Utilities|Array|IsEmpty _characters)
    (Development|PrintString "Game over")
    (Class|GameModeBase|ResetLevel)))

(event Custom|OnTurretDestroyed
  (params (DestroyedActor :type Actor%20Object%20Reference))
  (bind _turrets (Variables|Default|GetTurrets))
  ;[1 1 1] Remove turret from array on destroy
  (bind _asbp_turret (Utilities|Casting|CastToBP_Turret DestroyedActor))
  (Utilities|Array|RemoveItem _turrets _asbp_turret)
  (if (Utilities|Array|IsEmpty _turrets)
    (Utilities|String|LogString "Win")))

(event EventBeginPlay
  (Utilities|FlowControl|Sequence
    (:then_0
      ;[1 1 1] Create HUD
      (bind _returnvalue (UserInterface|CreateWidget "/Game/Game/Tests/Alexis/UI/HUD_Heatlh.HUD_Heatlh_C"))
      (UserInterface|Viewport|AddtoViewport _returnvalue 0))
    (:then_1
      ;[1 1 1] Get all turrets from level
      (bind _outactors (Actor|GetAllActorsOfClass "/Game/Game/Tests/Emilie/BP_Turret.BP_Turret_C"))
      (bind _output_get (Variables|Default|SetTurrets _outactors))
      (for _array_element _output_get
        (Game|BindEventtoOnDestroyed _array_element (delegate Custom|OnTurretDestroyed))))
    (:then_2
      (bind _outactors_2 (Actor|GetAllActorsOfClass "/Game/Game/Tests/Theo/Blueprints/Characters/BP_BaseCharacter.BP_BaseCharacter_C"))
      (bind _output_get_2 (Variables|Default|SetCharacters _outactors_2))
      (for _array_element_2 _output_get_2
        (EventDispatchers|BindEventtoOnDeath _array_element_2 (delegate Custom|OnCharacterDeath))))))

(fn ConstructionScript)

(fn AddCharacter)