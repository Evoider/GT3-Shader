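; Character Blueprint for "The Rusty Warrior", which adds a weapon slash trail and modular mesh setup on top of its parent class.
; On BeginPlay it attaches a Niagara trail to the right weapon, using the top and bottom trail sockets to set its midpoint, orientation and width.
; It also makes the hair, glove, shoe, shoulder pad and face follow the main mesh through leader pose, then sets the display name.
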(event EventBeginPlay
  (bind _rightweapon (Variables|Default|GetRightWeapon))
  (bind _returnvalue (Transformation|GetSocketLocation _rightweapon "Trail_01_Top"))
  (bind _returnvalue_2 (Transformation|GetSocketLocation _rightweapon "Trail_01_Bottom"))
  (bind _returnvalue_3 (- _returnvalue _returnvalue_2))
  (|CallParentFunction)
  (Utilities|FlowControl|Sequence
    (:then_0
      (bind _returnvalue_4 (Niagara|SpawnSystemAttached "/Game/Game/Alexis/Niagara/NS_SlashTrail.NS_SlashTrail" _rightweapon "None" (/ (+ _returnvalue _returnvalue_2) 2.0) (Math|Rotator|MakeRotfromZ _returnvalue_3) "KeepWorldPosition" false))
      (Effects|Components|ParticleSystem|SetFloatParameter _returnvalue_4 "TrailWidth" (Math|Vector|VectorLength _returnvalue_3)))
    (:then_1
      (Components|SkinnedMesh|SetLeaderPoseComponent (Variables|Default|GetHair) (Variables|Character|GetMesh) false false)
      (Variables|Default|SetName "The Rusty Warrior"))))

(fn ConstructionScript
  (|CallParentFunction))