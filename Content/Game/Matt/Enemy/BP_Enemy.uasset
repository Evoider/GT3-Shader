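; Enemy character that senses player characters, pursues them and attacks for fixed damage, with a health bar widget turned toward the camera.
; PawnSensing triggers an AI move toward the seen player's controller when out of range, attacking on success.
; Damage applies an overlay material, updates the health bar and, at zero health, flags death and starts a timer.
; JumpNavMesh turns the enemy and launches it along a computed arc to a destination.
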(event OnSeePawn(PawnSensing)
  (params (Pawn :type Pawn%20Object%20Reference))
  (if (not (Variables|Default|GetisDead))
    (bind _asbp_base_character (Utilities|Casting|CastToBP_BaseCharacter Pawn))
    (Utilities|FlowControl|Sequence
      (:then_0
        ;[1 1 1] Get Seen Player Character and Controller
        (bind _output_get (Variables|Default|SetPlayerCharacter _asbp_base_character))
        (bind _asbp_hero_controller (Utilities|Casting|CastToBP_HeroController (Pawn|GetController _output_get)))
        (Variables|Default|SetPlayerController _asbp_hero_controller))
      (:then_1
        (if (not (<= (Transformation|GetDistanceTo (Variables|Default|GetPlayerController)) (+ (Variables|Default|GetAttackingRange) 1e+02)))
          (AI|AIMoveTo self "0, 0, 0" (Variables|Default|GetPlayerController) 5.0 true
            (:OnSuccess
              (if (Variables|Default|GetIsAttacking)
                (Utilities|FlowControl|Delay 2.0))
              (CallFunction|Attack))))))))

(event Custom|OnEndHit
  (Variables|Default|SetIsHit false))

(event Custom|JumpNavMesh
  (params (Destination :type Vector))
  (bind (_x _y _z) (Math|Vector|BreakVector Destination))
  (Utilities|FlowControl|Sequence
    (:then_0
      ;[1 1 1] Doesn't work without it
      (Utilities|FlowControl|Delay 0.01)
      (Transformation|SetActorRotation (Math|Rotator|MakeRotator 0.0 0.0 (.yaw (Math|Rotator|FindLookatRotation (Transformation|GetActorLocation) Destination)))))
    (:then_1
      (bind _outlaunchvelocity (Game|SuggestProjectileVelocityCustomArc (Transformation|GetActorLocation) (Math|Vector|MakeVector _x _y (+ _z 2e+02)) 0.0 0.5))
      (Character|LaunchCharacter _outlaunchvelocity true true))))

(event EventTick
  (params (DeltaSeconds :type Float%20%28single-precision%29))
  (bind _widget (Variables|Default|GetWidget))
  (Transformation|SetWorldRotation _widget (Math|Rotator|FindLookatRotation (Transformation|GetWorldLocation _widget) (Transformation|GetWorldLocation (Variables|/Script/Engine.PlayerCameraManager|GetTransformComponent (Game|GetPlayerCameraManager 0)))) false false))

(event Game|Damage|EventAnyDamage
  (params (Damage :type Float%20%28single-precision%29) (DamageType :type Damage%20Type%20Object%20Reference) (InstigatedBy :type Controller%20Object%20Reference) (DamageCauser :type Actor%20Object%20Reference))
  (CallFunction|UpdateLife Damage)
  (Variables|Default|SetIsHit true))

(fn ConstructionScript)

(fn UpdateLife
  (params (Value :type Float%20%28double-precision%29))
  (Rendering|Material|SetOverlayMaterial (Variables|Character|GetMesh) "/Game/Game/Emilie/Materials/M_Damage.M_Damage" :!class /Script/Engine.MeshComponent)
  (bind _output_get (Variables|Default|SetCurrentHealth (- (Variables|Default|GetCurrentHealth) Value)))
  (Utilities|FlowControl|Sequence
    (:then_0
      (bind _ashud_ennemy_health (Utilities|Casting|CastToHUD_EnnemyHealth (UserInterface|GetWidget (Variables|Default|GetWidget))))
      (Default|UpdateHealthBar _ashud_ennemy_health (Variables|Default|GetCurrentHealth)))
    (:then_1
      (Utilities|Time|SetTimerbyEvent (EventDispatchers|CreateEvent :!event ResetOverlay) 0.1))
    (:then_2
      (if (<= _output_get 0.0)
        (Variables|Default|SetIsDead true)
        (Utilities|Time|SetTimerbyEvent (EventDispatchers|CreateEvent :!event Die) 3.0)))))

(fn Die
  (Actor|DestroyActor))

(fn DesactivateCollision
  (Collision|SetCollisionResponsetoChannel (Variables|Collision|GetCapsuleComponent) "ECC_GameTraceChannel1" "ECR_Ignore")
  (Collision|SetCollisionResponsetoChannel (Variables|Character|GetMesh) "ECC_WorldStatic" "ECR_Ignore")
  (Collision|SetCollisionResponsetoChannel (Variables|Collision|GetCapsuleComponent) "ECC_Pawn" "ECR_Ignore")
  (Collision|SetCollisionResponsetoChannel (Variables|Character|GetMesh) "ECC_Pawn" "ECR_Ignore"))

(fn IsDying)

(fn Attack
  (Variables|Default|SetIsAttacking true)
  (Default|Damage (Variables|Default|GetPlayerCharacter) 1e+01 false))

(fn ResetOverlay
  (Rendering|Material|SetOverlayMaterial (Variables|Character|GetMesh) 0 :!class /Script/Engine.MeshComponent))